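; Example actor for the RuntimeMeshLoader plugin that loads a textured gun from FBX and PNG files at runtime.
; Shortly after BeginPlay, it builds a dynamic material from diffuse and normal textures, then loads the mesh.
; Each node becomes a procedural mesh component attached by parent index, with relative transforms applied only to child nodes.
; The material is set only on element 0, and the delayed mesh cleanup chain is unwired.
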(event Custom|AttachToThisActor
  (params (ProcMeshComp :type Procedural%20Mesh%20Component%20Object%20Reference) (parentindex :type Integer) (RelativeTransform :type Transform))
  (bind _procmeshes (Variables|Default|GetProcMeshes))
  ;[1 1 1] Attach to this actor
  (Utilities|Array|Add _procmeshes ProcMeshComp)
  (if (< parentindex 0)
    (Transformation|AttachComponentToComponent ProcMeshComp (Variables|Default|GetDefaultSceneRoot) "None" "KeepRelative" "KeepRelative" "KeepRelative" true)
    (else
      (Transformation|AttachComponentToComponent ProcMeshComp (Utilities|Array|Get(acopy) _procmeshes parentindex) "None" "KeepRelative" "KeepRelative" "KeepRelative" true)
      (Transformation|SetRelativeTransform ProcMeshComp RelativeTransform false false))))

(event EventBeginPlay
  (bind _returnvalue (Class|KismetSystemLibrary|GetProjectDirectory))
  ;[1 1 1] load Texure2D from png file
  (Utilities|FlowControl|Delay 0.2)
  (bind (_isvalid _width _height _returnvalue_2) (Class|MeshLoader|LoadTexture2DfromFile (Utilities|String|Append _returnvalue "\\Plugins\\RuntimeMeshLoader\\Resources\\Gun\\Gun_T.png")))
  (if _isvalid
    (bind (_isvalid_2 _width_2 _height_2 _returnvalue_3) (Class|MeshLoader|LoadTexture2DfromFile (Utilities|String|Append _returnvalue "\\Plugins\\RuntimeMeshLoader\\Resources\\Gun\\Gun_N.png")))
    (if _isvalid_2
      (bind _returnvalue_4 (Rendering|Material|CreateDynamicMaterialInstance "/Game/RML_BaseMateria_ue420.RML_BaseMateria_ue420" "None" :!class /Script/Engine.KismetMaterialLibrary))
      (Rendering|Material|SetTextureParameterValue _returnvalue_4 "TextureParam" _returnvalue_2)
      (Rendering|Material|SetTextureParameterValue _returnvalue_4 "NormalParam" _returnvalue_3)
      (Variables|Default|SetMat _returnvalue_4)
      ;[1 1 1] load mesh from file
      (bind _returnvalue_5 (Class|MeshLoader|LoadMeshfromFile (Utilities|String|Append _returnvalue "\\Plugins\\RuntimeMeshLoader\\Resources\\Gun\\Gun.fbx") "Absolute"))
      (if (.success _returnvalue_5)
        (for _array_element (.nodes _returnvalue_5)
          (bind _returnvalue_6 (AddComponent|AddProceduralMeshComponent true))
          (CallFunction|AttachtoThisActor _returnvalue_6 (.nodeparentindex _array_element) (.relativetransformtransform _array_element))
          (for (_array_element_2 _array_index) (.meshes _array_element)
            (Class|ProceduralMeshComponent|CreateMeshSectionLinearColor _returnvalue_6 _array_index (.vertices _array_element_2) (.triangles _array_element_2) (.normals _array_element_2) (.uvs _array_element_2) 0 0 0 0 (.tangents _array_element_2) false)
            (Rendering|Material|SetMaterial _returnvalue_6 0 (Variables|Default|GetMat))))
        (else
          (Development|PrintString "error in load mesh"))))))

(fn ConstructionScript)